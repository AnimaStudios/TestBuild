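; Base projectile spell actor that flies, reports what it hits and cleans itself up.
; The construction script looks up SpellInfo in DT_Spells by its spell-name enum and applies speed and gravity scale to the projectile movement.
; Its collision box ignores the instigator, or owner as fallback, and hits fire OnProjectileImpact with impact effect and sound.
; On impact or lifetime timeout, the spell effect deactivates, then the actor is destroyed after a data-driven delay.
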(event `self.ReceiveBeginPlay`
  (bind _returnvalue (`self.GetInstigator`))
  (`PrimitiveComponent.IgnoreActorWhenMoving` (`self.Box Collision`) (select `bool` (`KismetSystemLibrary.IsValid` _returnvalue) :`false` (`self.GetOwner`) :`true` _returnvalue :!type "Actor Object Reference") true)
  (`KismetSystemLibrary.Delay` 15.0)
  (`ActorComponent.Deactivate` (`self.Spell`))
  (`KismetSystemLibrary.Delay` (`.Deactivate_31_EF2CFBD549508AC86EAE278A114B8CA2` (break `/Game/_CORE/Magic/S_Spell_Info` (`self.SpellInfo`))))
  (`self.K2_DestroyActor`))

(event `self.Box Collision.OnComponentHit`
  (params (HitComponent :type "PrimitiveComponent Object Reference") (OtherActor :type "Actor Object Reference") (OtherComp :type "PrimitiveComponent Object Reference") (NormalImpulse :type "Vector Structure") (Hit :type "HitResult Structure (by ref)"))
  (bind (_bblockinghit _binitialoverlap _time _distance _location) (`GameplayStatics.BreakHitResult` Hit))
  (`self.OnProjectileImpact` OtherActor Hit)
  (`NiagaraFunctionLibrary.SpawnSystemAtLocation` (`self.ImpactEffect`) _location)
  (`GameplayStatics.PlaySoundAtLocation` (`self.ImpactSound`) _location (struct) 1.0 1.0 0.0 null null null null)
  (`ActorComponent.Deactivate` (`self.Spell`))
  (`KismetSystemLibrary.Delay` (`.Deactivate_31_EF2CFBD549508AC86EAE278A114B8CA2` (break `/Game/_CORE/Magic/S_Spell_Info` (`self.SpellInfo`))))
  (`self.K2_DestroyActor`))

(fn `UserConstructionScript`
  (bind _projectilemovement (`self.ProjectileMovement`))
  (bind _returnvalue (`|GetDataTableRow` "/Game/_CORE/Magic/DT_Spells.DT_Spells" (`KismetStringLibrary.Conv_StringToName` (`|GetEnumeratorNameAsString` (`.SpellName_9_B78667114FDB009C3CD7718C75BC94ED` (break `/Game/_CORE/Magic/S_Spell_Info` (`self.SpellInfo`))))))
    (:`then`
      (bind _output_get (set `self.SpellInfo` _returnvalue))
      (bind (_spellclass _spellname _spelltype _spellimage _manacost _potency _price _speed _gravityscale) (break `/Game/_CORE/Magic/S_Spell_Info` _output_get))
      (set `ProjectileMovementComponent.InitialSpeed` _speed _projectilemovement)
      (set `ProjectileMovementComponent.MaxSpeed` _speed _projectilemovement)
      (set `ProjectileMovementComponent.ProjectileGravityScale` _gravityscale _projectilemovement))))