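; BP_Weapon is the equipment system's weapon actor, taking its appearance from item data.
; The construction script looks up the item's data table row and, when found, applies that row's static mesh to its mesh component.
; AttachActor casts the owner to BP_Devol_BaseCharacter and attaches the weapon to that character's mesh with snap-to-target rules.
; The event graph holds no active logic.
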(fn `AttachActor`
  (`self.K2_AttachToComponent` (`Character.Mesh` (cast `/Game/_CORE/Charcaters/BP_Devol_BaseCharacter` (`self.GetOwner`) :!pure true)) "None" "SnapToTarget" "SnapToTarget" "SnapToTarget"))

(fn `UserConstructionScript`
  (bind _itemdata (`self.ItemData`))
  (bind _returnvalue (`|GetDataTableRow` (break `DataTableRowHandle` (break `/Game/_CORE/EquipmentSystem/S_Slots` _itemdata)) (`.RowName` (break `DataTableRowHandle` (break `/Game/_CORE/EquipmentSystem/S_Slots` _itemdata))))
    (:`then`
      (`StaticMeshComponent.SetStaticMesh` (`self.StaticMesh`) (`.StaticMesh_16_144F0DB147CE8C013508F3B81CFA5755` (break `/Game/_CORE/EquipmentSystem/S_CharacterItems` _returnvalue))))))