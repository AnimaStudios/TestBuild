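; Water plane actor that, when PPMesh is enabled, builds a mesh-based post-process effect for its water volume in the construction script.
; A camera-projected quad gets scaled bounds to avoid culling and a dynamic material synced to wave height and surface Z.
; Material parameters confine it to the yaw-rotated water area and a height limit, with very large XY limits when Extender is on.
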(fn `UserConstructionScript`
  (locals (Scale :type "Float (double-precision)") (`Box Limits` :type "Vector Structure"))
  (bind _mesh (`self.Mesh`))
  (`/Engine/EditorBlueprintResources/StandardMacros.IsValid` _mesh
    (:`Is Valid`
      (set `local.Box Limits` (`.BoxExtent` (`KismetMathLibrary.BreakBoxSphereBounds` (`StaticMesh.GetBounds` _mesh))))
      (if (`self.PP Mesh`)
        (`self.Water PP` (`local.Scale`))))))

(fn `Water PP`
  (params (Size :type "Float (double-precision)"))
  (locals (WaterPPMaterial :type "MaterialInstanceDynamic Object Reference"))
  (bind _pp_z_axis_limiter (`self.PP Z-Axis Limiter`))
  (bind _waterppmaterial (`local.WaterPPMaterial`))
  (bind _pp_mesh_mat (`self.PP Mesh Mat`))
  (bind _size (`local.Size`))
  ;[1 1 1] that mesh is a 1 by 1 unit plane that uses the vertex shader to project itself right in front of the camera. Since we do not 'technically' move that component from the CPU's perspective, its bounds remains in place at (0,0,0) relative to the water actor, and thus if we no longer have that location in view, the CPU might think it no longer needs to be rendered and the mesh might disappear. To fix that we have to hack the bounds of that plane to trick the CPU into thinking it's as big as the water actor and it's always in view within that water volume. Now the depth is an issue. The mesh might still disappear if you dive way, way below the water surface so you might want to increase that 'SM_WaterSyst_PostProcessQuad' bounds negative Z extention in its static mesh asset settings. This has the downside of making the whole actor's bound quite large and focusing on the actor using 'F' key will zoom really far out... :(
  (`/Engine/EditorBlueprintResources/StandardMacros.IsValid` _pp_mesh_mat
    (:`Is Valid`
      (bind _returnvalue (`AddComponent|NODE_AddStaticMeshComponent-0` :`RelativeTransform` (`KismetMathLibrary.MakeTransform` (0.0 0.0 0.0))))
      (`PrimitiveComponent.SetBoundsScale` _returnvalue (`local.Size`))
      ;[1 1 1] create a dynamic material instance so we can specify our wave height multiplier so it's visually in 'sync' with the water material and reads the wave buffer the exact same way
      (bind _returnvalue_2 (`PrimitiveComponent.CreateDynamicMaterialInstance` _returnvalue 0 _pp_mesh_mat "None"))
      (bind _output_get (set `local.WaterPPMaterial` _returnvalue_2))
      (`MaterialInstanceDynamic.SetScalarParameterValue` _output_get "Waves - Height" (`self.Height`)) ; important to sample waves height the same way we do for the water material
      (`MaterialInstanceDynamic.SetScalarParameterValue` _output_get "Z" (.z (`self.K2_GetActorLocation`)))
      (if (`self.Extender`)
        ;[1 1 1] restrict the XY world locations at which the vertices of that post process mesh can be offset to appear in front of the screen (unless the water body has a far mesh), essentially limiting this post process mesh to the water's bound (according to its axis so you can rotate the water surface in yaw without issue). Also limit how far above the water surface the post process mesh is allowed to be drawn so we don't pay the cost of drawing it when we're way above the water. This kinda make it act like the bounds of a regular post process material
        (`MaterialInstanceDynamic.SetVectorParameterValue` _waterppmaterial "Bounds" (make `LinearColor` 100000.0 100000.0 _pp_z_axis_limiter))
        (else
          (`MaterialInstanceDynamic.SetVectorParameterValue` _waterppmaterial "Bounds" (make `LinearColor` (* _size (.x (`self.GetActorScale3D`))) (* (.y (`self.GetActorScale3D`)) _size) _pp_z_axis_limiter))))
      (`MaterialInstanceDynamic.SetVectorParameterValue` _waterppmaterial "Axis" (make `LinearColor` (.x (`self.GetActorForwardVector`)) (.y (`self.GetActorForwardVector`)) (.x (`self.GetActorRightVector`)) (.y (`self.GetActorRightVector`)))))))